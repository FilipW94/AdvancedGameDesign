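; BP_Laser is a laser beam actor that stretches to the first obstacle ahead and damages actors that overlap it.
; Each tick, a box trace on the Visibility channel runs forward up to LaserRange, and the hit distance or full range sets SMParent's world Z scale.
; Overlapping actors that implement BPI_Damageable receive a fixed damage message once per overlap begin.
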(event `ChangeLaserSize`
  (params (NewLaserLength :type "Float (double-precision)"))
  (bind _sm_parent (`self.SM_Parent`))
  (bind (_returnvalue_x _returnvalue_y) (`KismetMathLibrary.BreakVector` (`SceneComponent.K2_GetComponentScale` _sm_parent)))
  (`SceneComponent.SetWorldScale3D` _sm_parent (`KismetMathLibrary.MakeVector` _returnvalue_x _returnvalue_y NewLaserLength)))

(event `self.ReceiveActorBeginOverlap`
  (params (OtherActor :type "Actor Object Reference"))
  (if (`KismetSystemLibrary.DoesImplementInterface` OtherActor "/Game/BPI_Damageable.BPI_Damageable_C")
    (message `/Game/BPI_Damageable.DamageHasBeenTaken` OtherActor 15.0 self "NewEnumerator0")))

(event `self.ReceiveTick`
  (params (DeltaSeconds :type "Float (single-precision)"))
  (bind _returnvalue (`self.K2_GetActorLocation`))
  (bind _outhit (`KismetSystemLibrary.BoxTraceSingle` _returnvalue (+ _returnvalue (* (`KismetMathLibrary.GetForwardVector` (`self.K2_GetActorRotation`)) (`self.LaserRange`))) (0.0 0.0 0.0) (struct) "TraceTypeQuery1"))
  (`self.ChangeLaserSize` (`KismetMathLibrary.SelectFloat` (/ (+ (`.Distance` (`GameplayStatics.BreakHitResult` _outhit)) 1.0) 100.0) (/ (`self.LaserRange`) 100.0) (`GameplayStatics.BreakHitResult` _outhit))))

(fn `UserConstructionScript`)