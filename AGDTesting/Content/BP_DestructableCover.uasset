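; BP_DestructableCover is a cover actor that takes damage from lasers and boss projectiles through its ACHealthComponent.
; On BeginPlay it binds to the laser-begin dispatcher on BP_ThirdPersonGameMode, which re-arms a laser damage flag.
; The first laser hit applies the dealt damage and clears the flag, limiting it to one hit per laser event.
; Boss projectiles bypass the flag and apply fixed damage, ignoring the incoming amount.
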(event `self.ReceiveBeginPlay`
  (bind _asbp_third_person_game_mode (cast `/Game/ThirdPerson/Blueprints/BP_ThirdPersonGameMode` (`GameplayStatics.GetGameMode`)))
  (add `/Game/ThirdPerson/Blueprints/BP_ThirdPersonGameMode.LaserEventBegin` _asbp_third_person_game_mode (delegate `LaserEventBegin_Event`)))

(event `LaserEventBegin_Event`
  (set `self.CanBeDamagedByLaser` true))

(event `/Game/BPI_Damageable.DamageHasBeenTaken`
  (params (DamageDealt :type "Float (double-precision)") (DamageDealer :type "Actor Object Reference") (DamageType :type "/Game/E_DamageType Enum" :default "NewEnumerator0"))
  (switch `/Game/E_DamageType` DamageType
    (:`NewEnumerator0`
      (if (`self.CanBeDamagedByLaser`)
        (set `self.CanBeDamagedByLaser` false)
        (`/Game/Blueprints/ActorComponents/AC_HealthComponent.DamageActor` (`self.AC_HealthComponent`) DamageDealt)))
    (:`NewEnumerator1`
      (`/Game/Blueprints/ActorComponents/AC_HealthComponent.DamageActor` (`self.AC_HealthComponent`) 5.0))))

(fn `UserConstructionScript`)