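; BP_Projectile is a short-lived projectile that fires toward the player's position and deals damage on overlap.
; On BeginPlay it aims once at player character 0 at initial speed, passing a world-space direction to SetVelocityInLocalSpace, and sets a limited lifespan.
; Mesh overlap sends a fixed damage message through BPI_Damageable if the other actor implements it, and destroys the projectile either way.
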(event `self.ReceiveBeginPlay`
  (`self.SetProjectileTrajectory`)
  (`self.SetLifeSpan` 5.0))

(event `self.Projectile_Mesh.OnComponentBeginOverlap`
  (params (OverlappedComponent :type "PrimitiveComponent Object Reference") (OtherActor :type "Actor Object Reference") (OtherComp :type "PrimitiveComponent Object Reference") (OtherBodyIndex :type Integer) (bFromSweep :type Boolean) (SweepResult :type "HitResult Structure (by ref)"))
  (if (`KismetSystemLibrary.DoesImplementInterface` OtherActor "/Game/BPI_Damageable.BPI_Damageable_C")
    (message `/Game/BPI_Damageable.DamageHasBeenTaken` OtherActor 5.0 null "NewEnumerator1")
    (`self.K2_DestroyActor`)
    (else
      (`self.K2_DestroyActor`))))

(fn `SetProjectileTrajectory`
  (`ProjectileMovementComponent.SetVelocityInLocalSpace` (`self.ProjectileMovement`) (* (`KismetMathLibrary.Normal` (- (`self.K2_GetActorLocation` (`GameplayStatics.GetPlayerCharacter` 0)) (`self.K2_GetActorLocation`))) (`ProjectileMovementComponent.InitialSpeed` (`self.ProjectileMovement`)))))

(fn `UserConstructionScript`)