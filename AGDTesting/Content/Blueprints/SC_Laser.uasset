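; SC_Laser is a component that gives its owning actor a BP_Laser and controls whether that laser is active.
; SpawnLaser spawns the laser from a given transform, stores a reference and attaches it to the owner with KeepRelative rules, so that transform becomes an offset from the owner.
; ToggleLaser uses the stored reference to hide or show the laser, switching its SMParent collision off or on to match.
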(fn `SpawnLaser`
  (params (SpawnPosition :type "Transform Structure"))
  (bind _returnvalue (`|SpawnActorFromClass` "/Game/Laser/BP_Laser.BP_Laser_C" SpawnPosition "Undefined" "MultiplyWithRoot" null null))
  (bind _output_get (set `self.BP_LaserRef` _returnvalue))
  (`Actor.K2_AttachToActor` _output_get (`self.GetOwner`) "None" "KeepRelative" "KeepRelative" "KeepRelative" true))

(fn `Toggle Laser`
  (params (HideLaser :type Boolean))
  (bind _bp_laserref (`self.BP_LaserRef`))
  (bind _sm_parent (`/Game/Laser/BP_Laser.SM_Parent` _bp_laserref))
  (if HideLaser
    (`Actor.SetActorHiddenInGame` _bp_laserref true)
    (`PrimitiveComponent.SetCollisionEnabled` _sm_parent "NoCollision")
    (else
      (`Actor.SetActorHiddenInGame` _bp_laserref false)
      (`PrimitiveComponent.SetCollisionEnabled` _sm_parent "QueryAndPhysics"))))