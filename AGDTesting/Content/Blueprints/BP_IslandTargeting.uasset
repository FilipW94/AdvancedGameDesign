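; BP_IslandTargeting spawns destructible cover near whichever predefined pillar location is closest to the player.
; After BeginPlay records those locations, TargetPlayer moves and rebuilds the NavMesh at the nearest one.
; Timed random navigable-point picks, loosely filtered for spacing, fill an array that SpawnPillar turns into BP_DestructableCover actors.
; The pillar cleanup-and-retarget chain is disconnected from its empty DestroyPillars event, and nothing here calls the navmesh-growing event.
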(event `self.ReceiveBeginPlay`
  (`self.SetPillarLocations`)
  (`self.SetNavMeshSize`)
  (`KismetSystemLibrary.Delay` 2.0)
  (`self.TargetPlayer`))

(event `SlowlyIncreaseNavMeshSize`
  (bind _navmesh (`self.NavMesh`))
  (bind (_returnvalue_x _returnvalue_y) (`KismetMathLibrary.BreakVector` (+ (`self.GetActorScale3D` _navmesh) 1.0)))
  (if (and (<= _returnvalue_x 5.0) (<= _returnvalue_y 5.0))
    (`self.SetActorScale3D` _navmesh (`KismetMathLibrary.MakeVector` _returnvalue_x _returnvalue_y 2.0))
    (`KismetSystemLibrary.ExecuteConsoleCommand` "RebuildNavigation" null)
    (`KismetSystemLibrary.K2_SetTimerDelegate` (delegate `SlowlyIncreaseNavMeshSize`) 2.0)
    (else
      (`self.FindRandomPointInNavMesh`))))

(event `FindRandomPointInNavMesh`
  (bind _randomlocation (`NavigationSystemV1.K2_GetRandomLocationInNavigableRadius` (`self.K2_GetActorLocation` (`self.NavMesh`)) 400.0 null null :!label _label))
  (for _array_element (`self.NavMeshPositions`)
    (if (== _array_element _randomlocation :`ErrorTolerance` 100.0)
      (set `self.NewPositionFound` false)
      (else
        (set `self.NewPositionFound` true)
        (break))))
  (if (`self.NewPositionFound`)
    (if (<= (`KismetArrayLibrary.Array_Length` (`self.NavMeshPositions`)) 3)
      (`KismetSystemLibrary.DrawDebugSphere` _randomlocation 100.0 12 (struct :`R` 1.0 :`G` 1.0 :`B` 1.0 :`A` 1.0) 5.0 1.0)
      (`KismetArrayLibrary.Array_AddUnique` (`self.NavMeshPositions`) _randomlocation)
      (`KismetSystemLibrary.K2_SetTimerDelegate` (delegate `FindRandomPointInNavMesh`) 1.0)
      (else
        (`self.SpawnPillar`)))
    (else
      (goto _label))))

(event `SpawnPillar`
  (for _array_element (`self.NavMeshPositions`)
    (`|SpawnActorFromClass` "/Game/BP_DestructableCover.BP_DestructableCover_C" (`KismetMathLibrary.MakeTransform` _array_element (struct :`Pitch` 1.0 :`Yaw` 1.0 :`Roll` 1.0)) "Undefined" "MultiplyWithRoot" null null)
    (`KismetArrayLibrary.Array_Add` (`self.PillarArray`)))
  (`KismetArrayLibrary.Array_Clear` (`self.NavMeshPositions`))
  (`KismetSystemLibrary.PrintString` "Cubes have been spawned")
  (`KismetSystemLibrary.K2_SetTimerDelegate` (delegate `DestroyPillars`) 3.0))

(event `DestroyPillars`)

(fn `FindNearestPillar`
  (bind _playerposition (`self.GetPlayerLocation`))
  (for _array_element (`self.PillarLocations`)
    (bind _returnvalue (`KismetMathLibrary.Vector_Distance` _playerposition _array_element))
    (if (<= _returnvalue (`self.CurrentClosestRange`))
      (set `self.CurrentClosestRange` _returnvalue :!label _label)
      (set `self.CurrentClosestPillar` _array_element)
      (elif (== (`self.CurrentClosestRange`) 0.0)
        (goto _label)
        (else
          (`KismetSystemLibrary.PrintString` "Location is not closer")))))
  (`self.SetNavMeshPosition` (`self.CurrentClosestPillar`)))

(fn `GetPlayerLocation`
  (returns (PlayerPosition :type "Vector Structure"))
  (return (`self.K2_GetActorLocation` (`GameplayStatics.GetPlayerCharacter` 0))))

(fn `SetNavMeshPosition`
  (params (NewNavMeshPosition :type "Vector Structure"))
  (`self.K2_SetActorLocation` (`self.NavMesh`) NewNavMeshPosition false true)
  (`KismetSystemLibrary.ExecuteConsoleCommand` "RebuildNavigation" null)
  (set `self.CurrentClosestPillar` (0.0 0.0 0.0))
  (set `self.CurrentClosestRange` 0.0))

(fn `SetNavMeshSize`
  (`self.SetActorScale3D` (`self.NavMesh`) (`self.NavMeshActiveSize`))
  (`KismetSystemLibrary.ExecuteConsoleCommand` "RebuildNavigation" null))

(fn `SetPillarLocations`
  (bind _output_get (set `self.PillarLocations` (`|MakeArray` (`SceneComponent.K2_GetComponentLocation` (`self.PillarLocation`)) (`SceneComponent.K2_GetComponentLocation` (`self.PillarLocation2`)) (`SceneComponent.K2_GetComponentLocation` (`self.PillarLocation3`)) (`SceneComponent.K2_GetComponentLocation` (`self.PillarLocation1`)) (`SceneComponent.K2_GetComponentLocation` (`self.PillarLocation4`)))))
  (for _array_element _output_get
    (`KismetSystemLibrary.DrawDebugSphere` _array_element 100.0 12 (struct :`R` 1.0 :`G` 1.0 :`B` 1.0 :`A` 1.0) 5.0 1.0)))

(fn `TargetPlayer`
  (`self.FindNearestPillar`)
  (`self.FindRandomPointInNavMesh`))

(fn `UserConstructionScript`)