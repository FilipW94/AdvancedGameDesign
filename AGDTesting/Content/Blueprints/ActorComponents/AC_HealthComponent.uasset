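; AC_HealthComponent is an actor component that tracks health for its owning actor and destroys that actor when health runs out.
; It fills CurrentHealth from MaxHealth on BeginPlay, then DamageActor subtracts damage and calls ActorDied at zero or below.
; ActorDied prints debug text and destroys the owner.
; Player health widget creation and updates exist only as disconnected nodes, so no UI is driven.
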(event `self.ReceiveBeginPlay`
  (set `self.CurrentHealth` (`self.MaxHealth`)))

(fn `ActorDied`
  (bind _returnvalue (`self.GetOwner`))
  (`KismetSystemLibrary.PrintString` (`KismetSystemLibrary.GetDisplayName` _returnvalue))
  (`Actor.K2_DestroyActor` _returnvalue)
  (`KismetSystemLibrary.PrintString` "Handle death logic"))

(fn `DamageActor`
  (params (DamageDealt :type "Float (double-precision)"))
  (bind _output_get (set `self.CurrentHealth` (- (`self.CurrentHealth`) DamageDealt)))
  (if (<= _output_get 0.0)
    (`self.ActorDied`)))

(fn `UpdateHealthWidget`)