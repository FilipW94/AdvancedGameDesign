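; AC_AutoTurret is an actor component that makes a BP_Boss owner fire projectiles automatically.
; On BeginPlay it caches the boss reference and waits briefly before the first shot.
; Each shot spawns a BP_Projectile at the world location of the boss's ProjectileSpawnPosition, then re-arms a timer to fire again, stopping the loop if the spawn fails.
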(event `self.ReceiveBeginPlay`
  (bind _asbp_boss (cast `/Game/BossAI/BP_Boss` (`self.GetOwner`)))
  (set `self.BP_BossRef` _asbp_boss)
  (`KismetSystemLibrary.Delay` 2.0)
  (`self.FireProjectile`))

(event `FireProjectile`
  (bind _returnvalue (`|SpawnActorFromClass` "/Game/Blueprints/BP_Projectile.BP_Projectile_C" (`KismetMathLibrary.MakeTransform` (`self.SetNozzleTransform`)) "AlwaysSpawn" "MultiplyWithRoot" null null))
  (`/Engine/EditorBlueprintResources/StandardMacros.IsValid` _returnvalue
    (:`Is Valid`
      (`KismetSystemLibrary.PrintString` "Projectile fired from turret")
      (`KismetSystemLibrary.K2_SetTimerDelegate` (delegate `FireProjectile`) 1.0))
    (:`Is Not Valid`
      (`KismetSystemLibrary.PrintString` "Projectile Spawn failed"))))

(fn `SetNozzleTransform`
  (returns (ProjectileSpawnPosition :type "Vector Structure"))
  (return (`SceneComponent.K2_GetComponentLocation` (`/Game/BossAI/BP_Boss.ProjectileSpawnPosition` (`self.BP_BossRef`)))))