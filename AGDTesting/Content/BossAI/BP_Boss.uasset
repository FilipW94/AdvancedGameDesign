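; Boss actor that performs a rotating laser attack and takes laser damage through its health component.
; It spawns its laser and caches the player at start.
; An attack broadcasts a laser-begin event through the game mode, then chains a rotation timeline into a spin timeline, toggling the laser between phases and signalling completion.
; That broadcast re-arms a flag limiting laser damage to one hit per event.
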(event `self.ReceiveBeginPlay`
  (bind _sc_laser (`self.SC_Laser`))
  (`self.SetPlayerRef`)
  (`/Game/Blueprints/SC_Laser.SpawnLaser` _sc_laser (`SceneComponent.GetRelativeTransform` _sc_laser))
  (`/Game/Blueprints/SC_Laser.Toggle Laser` _sc_laser true)
  (bind _asbp_third_person_game_mode (cast `/Game/ThirdPerson/Blueprints/BP_ThirdPersonGameMode` (`GameplayStatics.GetGameMode`)))
  (bind _output_get (set `self.ThirdPersonGameModeRef` _asbp_third_person_game_mode))
  (add `/Game/ThirdPerson/Blueprints/BP_ThirdPersonGameMode.LaserEventBegin` _output_get (delegate `LaserEventBegin_Event`)))

(event `LaserEventBegin_Event`
  (set `self.CanBeDamagedByLaser` true))

(event `InitializeLaserAttack`
  (bind (_returnvalue_roll _returnvalue_pitch _returnvalue_yaw) (`KismetMathLibrary.BreakRotator` (`self.K2_GetActorRotation`)))
  (`/Game/ThirdPerson/Blueprints/BP_ThirdPersonGameMode.LaserEventBegin` (`self.ThirdPersonGameModeRef`))
  (bind (_direction _newtrack_0) (`Timeline|Timeline` :!via `PlayFromStart`)
    (:`Update`
      (`self.K2_SetActorRotation` (`KismetMathLibrary.RLerp` (`KismetMathLibrary.MakeRotator` 0.0 0.0 _returnvalue_yaw) (`KismetMathLibrary.MakeRotator` 0.0) _newtrack_0 true)))
    (:`Finished`
      (`/Game/Blueprints/SC_Laser.Toggle Laser` (`self.SC_Laser`) false)
      (`self.SpinInCircle`))))

(event `PrintPlayerHealthAndLocation`
  (`self.GetPlayerLocation`)
  (`KismetSystemLibrary.K2_SetTimerDelegate` (delegate `PrintPlayerHealthAndLocation`) 2.0))

(event `SpinInCircle`
  (bind (_direction _newtrack_0) (`Timeline|SpinTimeline` :!via `PlayFromStart`)
    (:`Update`
      (`self.K2_SetActorRotation` (`KismetMathLibrary.MakeRotator` 0.0 0.0 _newtrack_0)))
    (:`Finished`
      (`/Game/Blueprints/SC_Laser.Toggle Laser` (`self.SC_Laser`) true)
      (`self.LaserAttackDone`))))

(event `/Game/BPI_Damageable.DamageHasBeenTaken`
  (params (DamageDealt :type "Float (double-precision)") (DamageDealer :type "Actor Object Reference") (DamageType :type "/Game/E_DamageType Enum" :default "NewEnumerator0"))
  (switch `/Game/E_DamageType` DamageType
    (:`NewEnumerator0`
      (if (`self.CanBeDamagedByLaser`)
        (set `self.CanBeDamagedByLaser` false)
        (`/Game/Blueprints/ActorComponents/AC_HealthComponent.DamageActor` (`self.AC_HealthComponent`) DamageDealt)))))

(fn `GetPlayerLocation`
  (`KismetSystemLibrary.DrawDebugLine` (`SceneComponent.K2_GetComponentLocation` (`self.Nozzle`)) (`self.K2_GetActorLocation` (`self.PlayerRef`)) (struct :`R` 1.0 :`B` 0.11875 :`A` 1.0) 1.0 10.0)
  (return))

(fn `SetPlayerRef`
  (bind _outactors (`GameplayStatics.GetAllActorsOfClass` "/Game/ThirdPerson/Blueprints/BP_ThirdPersonCharacter.BP_ThirdPersonCharacter_C"))
  (for _array_element _outactors
    (bind _playerref (`/Game/FunctionLibrary.GetPlayerRef` _array_element))
    (bind _output_get (set `self.PlayerRef` _playerref))
    (`/Engine/EditorBlueprintResources/StandardMacros.IsValid` _output_get
      (:`Is Valid`
        (bind _output_get_2 (set `self.PlayerHealthComponentRef` (`/Game/ThirdPerson/Blueprints/BP_ThirdPersonCharacter.AC_HealthComponent` _output_get)))
        (`/Engine/EditorBlueprintResources/StandardMacros.IsValid` _output_get_2
          (:`Is Valid`
            (break))
          (:`Is Not Valid`
            (`KismetSystemLibrary.PrintString` "BP_Boss: Player health component not valid"))))
      (:`Is Not Valid`
        (`KismetSystemLibrary.PrintString` "BP_Boss: Player Ref not valid"))))
  (return))

(fn `UserConstructionScript`)